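; Harris 3D IK effector volume that supplies selected mesh vertices as hand and foot IK targets.
; A box, sized in construction, adds or removes the actor from an overlapping ThirdPersonCharacter's Harris list.
; Queries pick vertex indices by distance, with the Realistic variant taking the farthest within range and a direction cone.
; Getters turn indices into locations, normals and per-limb rotations; type is stubbed to BUMP, and normal and trace filters are disconnected.
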(event OnComponentBeginOverlap(Box)
  (params (OverlappedComponent :type Primitive%20Component%20Object%20Reference) (OtherActor :type Actor%20Object%20Reference) (OtherComp :type Primitive%20Component%20Object%20Reference) (OtherBodyIndex :type Integer) (bFromSweep :type Boolean) (SweepResult :type Hit%20Result%20Structure%20%28by%20ref%29))
  (bind _asthird_person_character (Utilities|Casting|CastToThirdPersonCharacter OtherActor))
  (Default|AddHarristoList _asthird_person_character self))

(event OnComponentEndOverlap(Box)
  (params (OverlappedComponent :type Primitive%20Component%20Object%20Reference) (OtherActor :type Actor%20Object%20Reference) (OtherComp :type Primitive%20Component%20Object%20Reference) (OtherBodyIndex :type Integer))
  (bind _asthird_person_character (Utilities|Casting|CastToThirdPersonCharacter OtherActor))
  (Default|DeleteHarrisfromList _asthird_person_character self))

(event EventBeginPlay)

(event Collision|EventActorBeginOverlap
  (params (OtherActor :type Actor%20Object%20Reference)))

(event EventTick
  (params (DeltaSeconds :type Float%20%28single-precision%29)))

(fn ConstructionScript
  (bind _boxcolliderscale (Variables|Default|GetBoxColliderScale))
  (bind _box (Variables|Default|GetBox))
  (Components|Box|SetBoxExtent _box _boxcolliderscale true)
  (Transformation|SetRelativeLocation _box (Math|Vector|MakeVector 0.0 0.0 (.Z (Math|Vector|BreakVector _boxcolliderscale))) false false))

(fn GetClosestEffector
  (params (inputLoc :type Vector) (inputPelvis :type Vector) (inputLimit_Max :type Float%20%28double-precision%29) (inputLimit_Min :type Float%20%28double-precision%29) (inputConditionDir :type Vector) (inputConditionDot :type Float%20%28double-precision%29))
  ;[1 1 1] 유효성 판단
  (if (<= (Utilities|Array|Length (Variables|Default|GetcurrentVrtLocs_postSelected)) 0)
    (return -1)
    (else
      ;[1 1 1] 초기화
      (LocalVariables|SetminDist 1e+03)
      (LocalVariables|SetcurtIndex -1)
      (LocalVariables|SetretLoc "0, 0, 0")
      ;[1 1 1] 반복
      (for (_array_element _array_index) (Variables|Default|GetcurrentVrtLocs_postSelected)
        ;[1 1 1] 조건 - 노멀
        (bind (_nor _bo) (CallFunction|GetEffectorNorbyIndex _array_index))
        (Development|PrintString (Utilities|String|ToString(Float) inputLimit_Max))
        (if (Math|Boolean|ANDBoolean (< (Math|Vector|Distance(Vector) _array_element inputLoc) inputLimit_Max) true true)
          ;[1 1 1] 가장 처음으로 하나 선택했을 때
          (if (== (LocalVariables|GetcurtIndex) -1)
            (LocalVariables|SetminDist (Math|Vector|Distance(Vector) (LocalVariables|GetretLoc) _array_element))
            (LocalVariables|SetretLoc _array_element)
            (LocalVariables|SetcurtIndex _array_index)
            (else
              ;[1 1 1] 미리 선택한 위치와 비교
              (if (< (Math|Vector|Distance(Vector) (LocalVariables|GetretLoc) _array_element) (LocalVariables|GetminDist))
                (LocalVariables|SetminDist (Math|Vector|Distance(Vector) (LocalVariables|GetretLoc) _array_element))
                (LocalVariables|SetretLoc _array_element)
                (LocalVariables|SetcurtIndex _array_index))))))
      ;[1 1 1] 마무리
      (return (LocalVariables|GetcurtIndex)))))

(fn GetClosestEffectorRealistic
  (params (inputLoc :type Vector) (inputDetectionDist :type Float%20%28double-precision%29) (inputDetectionDir :type Vector))
  ;[1 1 1] 유효성 판단
  (if (<= (Utilities|Array|Length (Variables|Default|GetcurrentVrtLocs_postSelected)) 0)
    (return -1)
    (else
      ;[1 1 1] 초기화
      (LocalVariables|SetmaxDist 0.0)
      (LocalVariables|SetcurtIndex -1)
      (LocalVariables|SetretLoc "0, 0, 0")
      ;[1 1 1] 반복
      (for (_array_element _array_index) (Variables|Default|GetcurrentVrtLocs_postSelected)
        ;[1 1 1] 조건 - 거리
        (bind _output_get (LocalVariables|SetinstDist (Math|Vector|Distance(Vector) _array_element inputLoc)))
        (bind _output_get_2 (LocalVariables|SetinstDot (Math|Vector|DotProduct (Math|Vector|Normalize (- _array_element inputLoc)) inputDetectionDir)))
        (if (and (< _output_get inputDetectionDist) (> _output_get_2 0.3))
          ;[1 1 1] 가장 처음으로 하나 선택했을 때
          (if (== (LocalVariables|GetcurtIndex) -1)
            (LocalVariables|SetretLoc _array_element :!label _label)
            (LocalVariables|SetcurtIndex _array_index)
            (LocalVariables|SetmaxDist (LocalVariables|GetinstDist))
            (else
              ;[1 1 1] 미리 선택한 위치와 비교
              (if (> (LocalVariables|GetinstDist) (LocalVariables|GetmaxDist))
                (goto _label))))))
      ;[1 1 1] 마무리
      (return (LocalVariables|GetcurtIndex)))))

(fn GetEffectorLocbyIndex
  (params (ind :type Integer))
  (if (!= ind -1)
    (return (Utilities|Array|Get(acopy) (Variables|Default|GetcurrentVrtLocs_postSelected) ind) true)
    (else
      (return "0, 0, 0" false))))

(fn GetEffectorNorbyIndex
  (params (ind :type Integer))
  (if (!= ind -1)
    (return (Utilities|Array|Get(acopy) (Variables|Default|GetcurrentVrtNors_postSelected) ind) true)
    (else
      (return "0, 0, 0" false))))

(fn GetEffectorRotbyIndexHandLeft
  (params (ind :type Integer) (forward :type Vector))
  (bind (_nor _bo) (CallFunction|GetEffectorNorbyIndex ind))
  (if _bo
    (bind _output_get (LocalVariables|Setnormal _nor))
    (return (Class|KismetMathLibrary|MakeRotfromYX _output_get forward) true)
    (else
      (return "0, 0, 0" false))))

(fn GetEffectorRotbyIndexHandRight
  (params (ind :type Integer) (forward :type Vector))
  (bind (_nor _bo) (CallFunction|GetEffectorNorbyIndex ind))
  (if _bo
    (bind _output_get (LocalVariables|Setnormal _nor))
    (return (Class|KismetMathLibrary|MakeRotfromYX (* _output_get -1.0) (* forward -1.0)) true)
    (else
      (return "0, 0, 0" false))))

(fn GetEffectorRotbyIndexFootLeft
  (params (ind :type Integer) (forward :type Vector))
  (bind (_nor _bo) (CallFunction|GetEffectorNorbyIndex ind))
  (if _bo
    (bind _output_get (LocalVariables|Setnormal _nor))
    (return (Math|Rotator|MakeRotfromXY _output_get (* forward -1.0)) true)
    (else
      (return "0, 0, 0" false))))

(fn GetEffectorRotbyIndexFootRight
  (params (ind :type Integer) (forward :type Vector))
  (bind (_nor _bo) (CallFunction|GetEffectorNorbyIndex ind))
  (if _bo
    (bind _output_get (LocalVariables|Setnormal _nor))
    (return (Math|Rotator|MakeRotfromXY (* _output_get -1.0) (* forward 1.0)) true)
    (else
      (return "0, 0, 0" false))))

(fn GetEffectorTypebyIndex
  (params (inputIndex :type Integer))
  (return "VERTEX_BUMP"))